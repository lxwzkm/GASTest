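; BP_FireBall is the Fire Blast ability's projectile, which flies out, returns to a target actor and explodes.
; On authority, two timelines lerp it forward to a maximum distance, then back toward ActorToReturn's current position.
; Within the explode distance, it calls OnHit, applies radial GAS damage to nearby live players except its owner, and destroys itself.
; Knockback pitch is overridden to 45 degrees, while death impulse points straight away from the blast.
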(event EventStartOutgoingTimeline
  (bind _returnvalue (Components|GetOwner))
  (bind _self self)
  (bind _array (Utilities|Array|MakeArray _returnvalue))
  (Networking|SwitchHasAuthority
    (:Authority
      ;[1 1 1] 获取起点与终点
      (Variables|Default|SetInitialLocation (Transformation|GetActorLocation))
      (Variables|Default|SetApexLocation (+ (Variables|Default|GetInitialLocation) (* (Transformation|GetActorForwardVector) (Variables|Default|GetMaxDIstance))))
      (bind _newtrack_0 (Timeline|OutgoingTimeline PlayFromStart)
        (:Update
          (Transformation|SetActorLocation (Math|Vector|Lerp(Vector) (Variables|Default|GetInitialLocation) (Variables|Default|GetApexLocation) _newtrack_0) false false))
        (:Finished
          (bind _newtrack_0_2 (Timeline|ReturnTimeline PlayFromStart)
            (:Update
              (Transformation|SetActorLocation (Math|Vector|Lerp(Vector) (Variables|Default|GetApexLocation) (Transformation|GetActorLocation (Variables|Default|GetActorToReturn)) _newtrack_0_2) false false)
              (if (<= (Math|Vector|VectorLength (- (Transformation|GetActorLocation) (Transformation|GetActorLocation (Variables|Default|GetActorToReturn)))) (Variables|Default|GetMinExplodeDistance))
                (Class|GASTProjectile|OnHit)
                (Class|GASTAbilitySystemLibrary|SetRadialDamageEffectParams (Variables|Default|GetDamageEffectParam) true (Variables|Default|GetRadial%20Inner%20Radius) (Variables|Default|GetRadial%20Outer%20Radius) (Transformation|GetActorLocation))
                (Utilities|Array|Add _array _self)
                (bind _outoverlapactors (Class|GASTAbilitySystemLibrary|GetLivePlayerswithinRadius _self _array (Variables|Default|GetRadial%20Outer%20Radius) (Transformation|GetActorLocation)))
                (for _array_element _outoverlapactors
                  (Class|GASTAbilitySystemLibrary|SetDamageParamsTargetASC (Variables|Default|GetDamageEffectParam) (Ability|GetAbilitySystemComponent _array_element))
                  (Variables|Default|SetDIrection (- (Transformation|GetActorLocation _array_element) (Transformation|GetActorLocation)))
                  (bind _returnvalue_2 (CallFunction|OverridePitch))
                  (Class|GASTAbilitySystemLibrary|SetKnockBackDirection (Variables|Default|GetDamageEffectParam) _returnvalue_2 8e+02)
                  (Class|GASTAbilitySystemLibrary|SetDeathImpulseDirection (Variables|Default|GetDamageEffectParam) (Variables|Default|GetDIrection) 6e+02)
                  (Class|GASTAbilitySystemLibrary|ApplyDamageEffecttoTarget (Variables|Default|GetDamageEffectParam)))
                (Actor|DestroyActor)))))))))

(fn ConstructionScript)

(fn OverridePitch
  (bind _direction (Variables|Default|GetDIrection))
  (bind _returnvalue (Math|Rotator|MakeRotfromX _direction))
  (return (Math|Vector|GetForwardVector (Math|Rotator|MakeRotator (.roll _returnvalue) 45.0 (.yaw _returnvalue)))))