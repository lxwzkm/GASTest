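; BP_FireBolt is the bolt actor for the player's Fire Bolt ability, exploding once it stops or slows.
; Each Tick, MakeGoToBoom measures the distance moved since the previous frame instead of relying on hit events.
; Below MinLengthToExplode, it plays an impact sound, spawns a Niagara explosion and destroys itself.
; A delayed sphere-collision enable is left unconnected; no damage or movement logic appears in these graphs.
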(event EventBeginPlay)

(event Collision|EventActorBeginOverlap
  (params (OtherActor :type Actor%20Object%20Reference)))

(event EventTick
  (params (DeltaSeconds :type Float%20%28single-precision%29))
  (CallFunction|MakeGotoBoom))

(fn ConstructionScript)

(fn MakeGotoBoom
  (Variables|Default|SetLastSecondLocation (Variables|Default|GetThisSecondLocation))
  (Variables|Default|SetThisSecondLocation (Transformation|GetActorLocation))
  (if (< (Math|Vector|VectorLength (- (Variables|Default|GetThisSecondLocation) (Variables|Default|GetLastSecondLocation))) (Variables|Default|GetMinLengthToExplode))
    (Audio|PlaySoundatLocation "/Game/Assets/Sounds/Abilities/FireBolt/sfx_FireBolt_Impact.sfx_FireBolt_Impact" (Variables|Default|GetThisSecondLocation) "0, 0, 0" 1.0 1.0 0.0 0 0 0 0)
    (Niagara|SpawnSystematLocation "/Game/Assets/Effects/Projectiles/FireExplosion/NS_FireExplosion1.NS_FireExplosion1" (Variables|Default|GetThisSecondLocation))
    (Actor|DestroyActor)))