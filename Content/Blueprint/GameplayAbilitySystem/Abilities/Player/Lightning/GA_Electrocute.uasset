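; Player lightning ability that channels an electrocute beam at the target under the mouse until input is released.
; A montage event starts the ShockLoop cue and a looping timer that commits cost and applies set-by-caller lightning damage, ending when cost fails.
; Hitting a combat target disables movement and chains beam cues to additional targets, which also take damage.
; Otherwise the cue sits on the avatar, so cleanup removes cues per case.
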(event Custom|CommitCostAndDamage
  (bind _returnvalue (Ability|CommitAbilityCost false))
  (if _returnvalue
    (CallFunction|ApplyDamage)
    (else
      (Utilities|Time|ClearandInvalidateTimerbyHandle (Variables|Default|GetCostTimerHandle))
      (CallFunction|BeforeEndAbility)
      (Ability|EndAbility))))

(event Ability|EventActivateAbility
  (if (Utilities|DoesObjectImplementInterface (Ability|GetAvatarActorfromActorInfo) "/Script/NewMagicLegend.CombatInterface")
    ;[0.2104 0.2231 1] 保存点击的数据
    (bind _datahandle (|TargetDataUnderMouse)
      (:ValiedData
        (Class|DamageBeamSpell|StoreMouseHitResult (Ability|TargetData|GetHitResultfromTargetData _datahandle))
        (Class|DamageBeamSpell|StoreOwnerVariables)
        (Utilities|FlowControl|Sequence
          (:then_0
            (Variables|/Script/Engine.PlayerController|SetbShowMouseCursor (Variables|Default|GetOwnerPlayerController) false)
            (Class|CombatInterface|UpdateWarppingTarget(Message) (Ability|GetAvatarActorfromActorInfo) (Variables|Default|GetMouseHitLocation))
            (GameplayCue|ExecuteGameplayCue :GameplayCueTag "(TagName=\"GameplayCue.ShockBurst\")")
            (|PlayMontageandWaitProxy "None" (Variables|Default|GetMontage_Electrocute) 1.0 "None" true 1.0 0.0 false
              (:then
                (Ability|Tasks|WaitGameplayEvent "(TagName=\"Event.Montage.Electrocute\")" 0 true
                  (:EventReceived
                    (Class|CombatInterface|SetinShockLoop(Message) (Ability|GetAvatarActorfromActorInfo) true)
                    (CallFunction|SpawnElectrocuteBeam)
                    (bind _returnvalue (Utilities|Time|SetTimerbyEvent (delegate Custom|CommitCostAndDamage) (Variables|Default|GetCostFrequency) true))
                    (Variables|Default|SetCostTimerHandle _returnvalue))))))
          (:then_1
            (Ability|Tasks|WaitInputRelease false
              (:OnRelease
                (CallFunction|BeforeEndAbility)
                (Ability|EndAbility)))))))))

(event Ability|EventOnEndAbility
  (params (bWasCancelled :type Boolean)))

(fn BeforeEndAbility
  (Variables|/Script/Engine.PlayerController|SetbShowMouseCursor (Variables|Default|GetOwnerPlayerController) true)
  (Class|CombatInterface|SetinShockLoop(Message) (Ability|GetAvatarActorfromActorInfo) false)
  (Pawn|Components|CharacterMovement|SetMovementMode (Variables|/Script/Engine.Character|GetCharacterMovement (Variables|Default|GetOwnerCharacter)) "MOVE_Walking" 0)
  ;[1 1 1] 因为鼠标点击的结果不同，GC的所属也不一样，所以要分开处理
  (if (Variables|Default|GetFirstTargetHasInterface)
    (GameplayCue|RemoveGameplayCueOnActor(Looping) (Variables|Default|GetMouseHitActor) "(TagName=\"GameplayCue.ShockLoop\")" (Variables|Default|GetFirstGameplayCueParameters))
    (for _array_element (Variables|Default|GetOut%20Additional%20Targets)
      (if (.ReturnValue (Utilities|Map|Find (Variables|Default|GetAdditionalActorToCueParameters) _array_element))
        (GameplayCue|RemoveGameplayCueOnActor(Looping) _array_element "(TagName=\"GameplayCue.ShockLoop\")" (.Value (Utilities|Map|Find (Variables|Default|GetAdditionalActorToCueParameters) _array_element)))))
    (else
      (GameplayCue|RemoveGameplayCueOnActor(Looping) (Ability|GetAvatarActorfromActorInfo) "(TagName=\"GameplayCue.ShockLoop\")" (Variables|Default|GetFirstGameplayCueParameters)))))

(fn SpawnElectrocuteBeam
  (Class|DamageBeamSpell|TraceFirstActor (Variables|Default|GetMouseHitLocation))
  (bind _returnvalue (Class|CombatInterface|GetWeaponComponent(Message) (Ability|GetAvatarActorfromActorInfo)))
  (Variables|Default|SetFirstGameplayCueParameters (Ability|GameplayCue|MakeGameplayCueParameters :Location (Variables|Default|GetMouseHitLocation) :SourceObject (Variables|Default|GetMouseHitActor) :TargetAttachComponent _returnvalue))
  ;[1 1 1] 判断鼠标点击的是不是Enemy，是的话就将GC设置在Enemy上，不是就设置在玩家的Avatar上
  (bind _output_get (Variables|Default|SetFirstTargetHasInterface (Utilities|DoesObjectImplementInterface (Variables|Default|GetMouseHitActor) "/Script/NewMagicLegend.CombatInterface")))
  (if _output_get
    (Variables|Default|SetCueTarget (Variables|Default|GetMouseHitActor))
    (else
      (Variables|Default|SetCueTarget (Ability|GetAvatarActorfromActorInfo))))
  (GameplayCue|AddGameplayCueOnActor(Looping) (Variables|Default|GetCueTarget) "(TagName=\"GameplayCue.ShockLoop\")" (Variables|Default|GetFirstGameplayCueParameters))
  (if (Variables|Default|GetFirstTargetHasInterface)
    (bind _outadditionaltargets (Class|DamageBeamSpell|StoreAdditionalTargets))
    (bind _output_get_2 (Variables|Default|SetOut%20Additional%20Targets _outadditionaltargets))
    (for _array_element _output_get_2
      (CallFunction|AddShockLoopCuetoAdditionalParams _array_element))
    (Pawn|Components|CharacterMovement|DisableMovement (Variables|/Script/Engine.Character|GetCharacterMovement (Variables|Default|GetOwnerCharacter)))))

(fn AddShockLoopCuetoAdditionalParams
  (params (AdditionalActors :type Actor%20Object%20Reference))
  (LocalVariables|SetL_AdditionalTarget AdditionalActors)
  (Utilities|Map|Add (Variables|Default|GetAdditionalActorToCueParameters) (LocalVariables|GetL_AdditionalTarget) (Ability|GameplayCue|MakeGameplayCueParameters :Location (Transformation|GetActorLocation (LocalVariables|GetL_AdditionalTarget)) :SourceObject (LocalVariables|GetL_AdditionalTarget) :TargetAttachComponent (Variables|/Script/Engine.Actor|GetRootComponent (Variables|Default|GetMouseHitActor))))
  (GameplayCue|AddGameplayCueOnActor(Looping) (LocalVariables|GetL_AdditionalTarget) "(TagName=\"GameplayCue.ShockLoop\")" (Ability|GameplayCue|MakeGameplayCueParameters :Location (Transformation|GetActorLocation (LocalVariables|GetL_AdditionalTarget)) :SourceObject (LocalVariables|GetL_AdditionalTarget) :TargetAttachComponent (Variables|/Script/Engine.Actor|GetRootComponent (Variables|Default|GetMouseHitActor)))))

(fn ApplyDamage
  (CallFunction|ApplyDamageSignle (Variables|Default|GetMouseHitActor))
  (for _array_element (Variables|Default|GetOut%20Additional%20Targets)
    (CallFunction|ApplyDamageSignle _array_element)))

(fn ApplyDamageSignle
  (params (Actor :type Actor%20Object%20Reference))
  (bind _returnvalue (Ability|GetAbilitySystemComponentfromActorInfo))
  (bind _returnvalue_2 (Ability|GameplayEffect|AssignTagSetbyCallerMagnitude (GameplayEffects|MakeOutgoingSpec _returnvalue (Variables|Default|GetDamageEffectClass) (Math|Conversions|ToFloat(Integer) (Ability|GetAbilityLevel)) (GameplayEffects|MakeEffectContext _returnvalue)) "(TagName=\"Damage.Lightning\")" (Class|DamageGameplayAbility|GetDamageatLevel)))
  (GameplayEffects|ApplyGameplayEffectSpecToSelf (Ability|GetAbilitySystemComponent Actor) _returnvalue_2))