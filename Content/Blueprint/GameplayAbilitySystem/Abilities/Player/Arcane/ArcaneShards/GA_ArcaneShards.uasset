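; Arcane Shards player ability that, after a cost check, shows a magic circle and waits for input to target the point under the mouse.
; It spawns a point collection for level-scaled, randomly rotated ground points, then plays a warp-targeted cast montage.
; The montage event commits cost and starts a looping timer that fires a cue and radial knockback damage per point.
; After the last point, it commits cooldown and ends.
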(event Custom|SpawnPoint
  (bind _returnvalue (Ability|GetAvatarActorfromActorInfo))
  ;[1 1 1] 设置定时器重复生成特效并结束技能
  (if (< (Variables|Default|GetIndex) (Variables|Default|GetNum%20Points))
    (Variables|Default|SetPointsLocation (Transformation|GetWorldLocation (Utilities|Array|Get(acopy) (Variables|Default|GetCollectionPoints) (Variables|Default|GetIndex))))
    (bind _outoverlapactors (Class|GASTAbilitySystemLibrary|GetLivePlayerswithinRadius _returnvalue (Utilities|Array|MakeArray _returnvalue) (Variables|Default|GetRadialDamageOuterRadius) (Variables|Default|GetPointsLocation)))
    (for _array_element _outoverlapactors
      (Class|GASTAbilitySystemLibrary|ApplyDamageEffecttoTarget (Class|DamageGameplayAbility|MakeDamageParams _array_element (Variables|Default|GetPointsLocation) true (- (Transformation|GetActorLocation _array_element) (Variables|Default|GetPointsLocation)) true (- (Transformation|GetActorLocation _array_element) (Variables|Default|GetPointsLocation)) true 35.0)))
    (Math|Integer|IncrementInt (Variables|Default|GetIndex)
      (:%20%20
        (Class|GameplayAbility|ExecuteGameplayCuewithParams "(TagName=\"GameplayCue.ArcaneShards\")" (Ability|GameplayCue|MakeGameplayCueParameters :Location (Variables|Default|GetPointsLocation)))))
    (else
      (Utilities|Time|ClearandInvalidateTimerbyHandle (Variables|Default|GetSpawnPointsTimer))
      (Actor|DestroyActor (Variables|Default|GetPointCollectionActor))
      (Ability|CommitAbilityCooldown false)
      (Ability|EndAbility))))

(event Ability|EventActivateAbility
  (bind _returnvalue (Class|GameplayAbility|CheckAbilityCost))
  (if _returnvalue
    (Utilities|FlowControl|Sequence
      (:then_0
        ;[1 1 1] 生成魔法环
        (Class|PlayerInterface|ShowMagicCircle(Message) (Ability|GetAvatarActorfromActorInfo) 0))
      (:then_1
        ;[1 1 1] 获取鼠标点击数据
        (Ability|Tasks|WaitInputPress false
          (:OnPress
            (bind _datahandle (|TargetDataUnderMouse)
              (:ValiedData
                (Variables|Default|SetImpact%20Point (.ImpactPoint (Collision|BreakHitResult (Ability|TargetData|GetHitResultfromTargetData _datahandle))))
                (Utilities|FlowControl|Sequence
                  (:then_0
                    ;[1 1 1] 生成目标点
                    (bind _returnvalue_2 (Game|SpawnActorfromClass "/Game/Blueprint/GameplayAbilitySystem/Abilities/Player/Arcane/ArcaneShards/BP_PointCollection.BP_PointCollection_C" (Math|Transform|MakeTransform (Variables|Default|GetImpact%20Point) "0, 0, 0" "1.000000,1.000000,1.000000") "AlwaysSpawn" "MultiplyWithRoot" 0 0))
                    (bind _output_get (Variables|Default|SetPointCollectionActor _returnvalue_2))
                    (Variables|Default|SetNum%20Points (Math|Integer|Min(Integer) (Variables|Default|GetMaxSpawnNum) (Ability|GetAbilityLevel)))
                    (Variables|Default|SetCollectionPoints (Class|PointCollection|GetGroundPoints _output_get (Variables|Default|GetImpact%20Point) (Variables|Default|GetNum%20Points) (Math|Random|RandomFloatinRange 0.0 3.6e+02))))
                  (:then_1
                    ;[1 1 1] 更新施法朝向
                    (Class|CombatInterface|UpdateWarppingTarget(Message) (Ability|GetAvatarActorfromActorInfo) (Variables|Default|GetImpact%20Point)))
                  (:then_2
                    ;[1 1 1] 播放施法动作
                    (|PlayMontageandWaitProxy "None" "/Game/Assets/Characters/Aura/Animations/Abilities/AM_Cast_ArcaneShards.AM_Cast_ArcaneShards" 1.0 "None" false 1.0 0.0 false
                      (:then
                        (Ability|Tasks|WaitGameplayEvent "(TagName=\"Event.Montage.ArcaneShards\")" 0 true
                          (:EventReceived
                            ;[1 1 1] 设置定时器重复生成特效并结束技能
                            (bind _returnvalue_3 (Utilities|Time|SetTimerbyEvent (delegate Custom|SpawnPoint) (Variables|Default|GetSpawnPointsFrequency) true))
                            (Variables|Default|SetSpawnPointsTimer _returnvalue_3)
                            (CallFunction|SpawnPoint)
                            (Class|PlayerInterface|HideMagicCircle(Message) (Ability|GetAvatarActorfromActorInfo))
                            (Ability|CommitAbilityCost false)))))))))))))))

(event Ability|EventOnEndAbility
  (params (bWasCancelled :type Boolean)))