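; Gameplay ability for a melee attack: aims motion warping at the avatar's combat target and plays a random attack montage from its tagged montage list.
; A montage gameplay event triggers a small sphere query at the tag's weapon socket, damaging living non-friends and ending the ability.
; Montage completion, interruption or cancellation also ends it.
; Random indices are rolled separately for montage, event tag and socket, so they can mismatch.
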(event Ability|EventActivateAbility
  (bind _returnvalue (Ability|GetAvatarActorfromActorInfo))
  (bind _returnvalue_2 (Ability|GetAvatarActorfromActorInfo))
  (bind _ascombat_interface (Utilities|Casting|CastToCombatInterface _returnvalue_2))
  (bind _returnvalue_3 (Class|EnemyInterface|GetCombatTarget(Message) _returnvalue_2))
  (Class|CombatInterface|UpdateWarppingTarget _ascombat_interface (Transformation|GetActorLocation _returnvalue_3))
  (bind _returnvalue_4 (Class|CombatInterface|GetTagMontages _ascombat_interface))
  (|PlayMontageandWaitProxy "None" (.AttackMontage (Utilities|Struct|BreakTagMontage (Utilities|Array|Get(acopy) _returnvalue_4 (Math|Random|RandomIntegerinRange 0 (- (Utilities|Array|Length _returnvalue_4) 1))))) 1.0 "None" true 1.0 0.0 false
    (:then
      (Ability|Tasks|WaitGameplayEvent (.MontageTag (Utilities|Struct|BreakTagMontage (Utilities|Array|Get(acopy) _returnvalue_4 (Math|Random|RandomIntegerinRange 0 (- (Utilities|Array|Length _returnvalue_4) 1))))) 0
        (:EventReceived
          (bind _returnvalue_5 (Class|CombatInterface|GetWeaponSocketLocation(Message) _returnvalue (.MontageTag (Utilities|Struct|BreakTagMontage (Utilities|Array|Get(acopy) _returnvalue_4 (Math|Random|RandomIntegerinRange 0 (- (Utilities|Array|Length _returnvalue_4) 1)))))))
          (bind _outoverlapactors (Class|GASTAbilitySystemLibrary|GetLivePlayerswithinRadius _returnvalue (Utilities|Array|MakeArray _returnvalue) 45.0 _returnvalue_5))
          (for _array_element _outoverlapactors
            (if (Class|GASTAbilitySystemLibrary|IsNotFriend (Ability|GetAvatarActorfromActorInfo) _array_element)
              (Class|DamageGameplayAbility|CauseDamagetoTarget _array_element)))
          (Ability|EndAbility))))
    (:OnCompleted
      (Ability|EndAbility :!label _label))
    (:OnInterrupted
      (goto _label))
    (:OnCancelled
      (goto _label))))

(event Ability|EventOnEndAbility
  (params (bWasCancelled :type Boolean)))