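; Fire Bolt gameplay ability that casts a projectile at the location under the mouse cursor.
; On activation it gets cursor target data and passes the hit location to the avatar's CombatInterface as the warping target.
; It plays the cast montage at half speed and waits for the montage's gameplay event to time the projectile spawn.
; The ability ends only on the montage's Completed callback.
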(event Ability|EventActivateAbility
  (bind _datahandle (|TargetDataUnderMouse)
    (:ValiedData
      (Variables|Default|SetTargetDataLocation (.Location (Collision|BreakHitResult (Ability|TargetData|GetHitResultfromTargetData _datahandle))))
      (bind _ascombat_interface (Utilities|Casting|CastToCombatInterface (Ability|GetAvatarActorfromActorInfo)))
      (Class|CombatInterface|UpdateWarppingTarget _ascombat_interface (Variables|Default|GetTargetDataLocation))
      (|PlayMontageandWaitProxy "None" "/Game/Assets/Characters/Aura/Animations/Abilities/AM_Cast_FireBolt.AM_Cast_FireBolt" 0.5 "None" true 1.0 0.0 false
        (:then
          (Ability|Tasks|WaitGameplayEvent "(TagName=\"Event.Montage.FireBolt\")" 0
            (:EventReceived
              (Class|AbilityProjectileSpell|SpawnPrijectile (Variables|Default|GetTargetDataLocation)))))
        (:OnCompleted
          (Ability|EndAbility))))))

(event Ability|EventOnEndAbility
  (params (bWasCancelled :type Boolean)))