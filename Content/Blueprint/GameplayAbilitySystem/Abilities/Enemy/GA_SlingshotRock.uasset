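; Enemy Gameplay Ability for a slingshot rock attack on the avatar's combat target.
; It updates the motion warping target, plays a random tagged attack montage and waits for a montage tag event.
; That event applies damage directly to the target and ends the ability, while the projectile spawn is left unconnected.
; The montage and awaited tag come from separate random picks, so they can differ.
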(event Ability|EventActivateAbility
  (bind _returnvalue (Ability|GetAvatarActorfromActorInfo))
  (bind _ascombat_interface (Utilities|Casting|CastToCombatInterface _returnvalue))
  (bind _returnvalue_2 (Class|EnemyInterface|GetCombatTarget(Message) _returnvalue))
  (Class|CombatInterface|UpdateWarppingTarget _ascombat_interface (Transformation|GetActorLocation _returnvalue_2))
  (bind _returnvalue_3 (Class|CombatInterface|GetTagMontages _ascombat_interface))
  (|PlayMontageandWaitProxy "None" (.AttackMontage (Utilities|Struct|BreakTagMontage (Class|DamageGameplayAbility|GetRandomTagMontage _returnvalue_3))) 1.0 "None" false 1.0 0.0 false
    (:then
      (Ability|Tasks|WaitGameplayEvent (.MontageTag (Utilities|Struct|BreakTagMontage (Class|DamageGameplayAbility|GetRandomTagMontage _returnvalue_3))) 0 true
        (:EventReceived
          (bind _returnvalue_4 (Class|EnemyInterface|GetCombatTarget(Message) (Ability|GetAvatarActorfromActorInfo)))
          (Class|GASTAbilitySystemLibrary|ApplyDamageEffecttoTarget (Class|DamageGameplayAbility|MakeDamageParams _returnvalue_4))
          (Ability|EndAbility))))))

(event Ability|EventOnEndAbility
  (params (bWasCancelled :type Boolean)))