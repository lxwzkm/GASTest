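; Enemy melee attack gameplay ability that warps toward the combat target and plays a randomly chosen tagged attack montage.
; The chosen montage entry is cached so the socket lookup matches the animation played.
; On the montage's gameplay event, it sphere-checks live players around that weapon socket and applies damage effects to non-friends.
; Any hit triggers a MeleeImpact gameplay cue at the socket, then the ability ends.
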(event Ability|EventActivateAbility
  (bind _returnvalue (Ability|GetAvatarActorfromActorInfo))
  (bind _returnvalue_2 (Ability|GetAvatarActorfromActorInfo))
  (Variables|Default|SetIsHeart false)
  (bind _ascombat_interface (Utilities|Casting|CastToCombatInterface _returnvalue_2))
  (bind _returnvalue_3 (Class|EnemyInterface|GetCombatTarget(Message) _returnvalue_2))
  (Class|CombatInterface|UpdateWarppingTarget _ascombat_interface (Transformation|GetActorLocation _returnvalue_3))
  (bind _returnvalue_4 (Class|CombatInterface|GetTagMontages _ascombat_interface))
  ;[1 1 1] 必须存起来，不然播放完蒙太奇后的GetWeaponSocketLocation会再次触发随机数，可能会获得不同的Tag，导致判断重叠的位置错误
  (bind _output_get (Variables|Default|SetTagMontage (Class|DamageGameplayAbility|GetRandomTagMontage _returnvalue_4)))
  (|PlayMontageandWaitProxy "None" (.AttackMontage (Utilities|Struct|BreakTagMontage _output_get)) 1.0 "None" false 1.0 0.0 false
    (:then
      (Ability|Tasks|WaitGameplayEvent (.MontageTag (Utilities|Struct|BreakTagMontage _output_get)) 0
        (:EventReceived
          (bind _returnvalue_5 (Class|CombatInterface|GetWeaponSocketLocation(Message) _returnvalue (.CombateTag (Utilities|Struct|BreakTagMontage _output_get))))
          (bind _outoverlapactors (Class|GASTAbilitySystemLibrary|GetLivePlayerswithinRadius _returnvalue (Utilities|Array|MakeArray _returnvalue) 45.0 _returnvalue_5))
          (for _array_element _outoverlapactors
            (if (Class|GASTAbilitySystemLibrary|IsNotFriend (Ability|GetAvatarActorfromActorInfo) _array_element)
              (Variables|Default|SetIsHeart true)
              (Class|GASTAbilitySystemLibrary|ApplyDamageEffecttoTarget (Class|DamageGameplayAbility|MakeDamageParams _array_element))))
          (if (Variables|Default|GetIsHeart)
            (Class|GameplayAbility|ExecuteGameplayCuewithParams "(TagName=\"GameplayCue.MeleeImpact\")" (Ability|GameplayCue|MakeGameplayCueParameters :AggregatedSourceTags (GameplayTags|MakeGameplayTagContainerfromTag (.MontageTag (Utilities|Struct|BreakTagMontage (Variables|Default|GetTagMontage)))) :Location _returnvalue_5 :EffectCauser (Ability|GetAvatarActorfromActorInfo) :SourceObject _array_element)))
          (Ability|EndAbility))))
    (:OnCompleted
      (Ability|EndAbility :!label _label))
    (:OnInterrupted
      (goto _label))
    (:OnCancelled
      (goto _label))))