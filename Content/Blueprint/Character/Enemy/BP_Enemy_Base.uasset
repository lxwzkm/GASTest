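; Base enemy character Blueprint that handles spawn scaling, facing-target updates and dissolve visuals.
; On BeginPlay a timeline animates the mesh's relative scale.
; UpdateWarppingTarget feeds a location into the MotionWarping component's FacingTarget warp target.
; StartDissove and WeaponStartDissove use separate timelines to drive the Dissolve scalar on the dynamic material passed in, for body and weapon respectively.
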(event EventBeginPlay
  (bind _newtrack_0 (Timeline|SpawnTimeLine Play)
    (:Update
      (Transformation|SetRelativeScale3D (Variables|Character|GetMesh) (Math|Conversions|ToVector(Float) _newtrack_0)))))

(event Collision|EventActorBeginOverlap
  (params (OtherActor :type Actor%20Object%20Reference)))

(event EventTick
  (params (DeltaSeconds :type Float%20%28single-precision%29)))

(event EventStartDissove
  (params (DynamicMaterila :type Material%20Instance%20Dynamic%20Object%20Reference))
  (bind _newtrack_0 (Timeline|MeshDissove Play)
    (:Update
      (Rendering|Material|SetScalarParameterValue DynamicMaterila "Dissolve" _newtrack_0 :!class /Script/Engine.MaterialInstanceDynamic))))

(event EventWeaponStartDissove
  (params (DynamicMaterila :type Material%20Instance%20Dynamic%20Object%20Reference))
  (bind _newtrack_0 (Timeline|WeaponDissove Play)
    (:Update
      (Rendering|Material|SetScalarParameterValue DynamicMaterila "Dissolve" _newtrack_0 :!class /Script/Engine.MaterialInstanceDynamic))))

(event EventUpdateWarppingTarget
  (params (TargetLocation :type Vector%20%28by%20ref%29 :default "0, 0, 0"))
  (Class|MotionWarpingComponent|AddorUpdateWarpTargetfromLocation (Variables|Default|GetMotionWarping) "FacingTarget" TargetLocation))

(fn ConstructionScript)