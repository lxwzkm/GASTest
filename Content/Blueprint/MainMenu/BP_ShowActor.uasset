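; BP_ShowActor is the main menu scene actor that opens WBP_MainMenu and animates a showcase fireball and magic circle.
; On BeginPlay it records the fireball's position, adds the menu widget to the viewport, sets UI-only input and shows the cursor.
; Each tick, UpdateTime advances a timer that resets at 2π, driving a sine bob of the fireball along Z, while the magic circle slowly rolls.
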(event EventBeginPlay
  (bind _returnvalue (Game|GetPlayerController 0))
  (Variables|Default|SetInitialLocation (Transformation|GetWorldLocation (Variables|Default|GetFIreBall)))
  (bind _returnvalue_2 (UserInterface|CreateWidget "/Game/Blueprint/UI/MainMenu/WBP_MainMenu.WBP_MainMenu_C"))
  (UserInterface|Viewport|AddtoViewport _returnvalue_2 0)
  (Input|SetInputModeUIOnly _returnvalue _returnvalue_2 "DoNotLock" false)
  (Variables|/Script/Engine.PlayerController|SetbShowMouseCursor _returnvalue true))

(event EventTick
  (params (DeltaSeconds :type Float%20%28single-precision%29))
  (CallFunction|UpdateTime DeltaSeconds)
  (Transformation|SetWorldLocation (Variables|Default|GetFIreBall) (+ (Variables|Default|GetInitialLocation) (Math|Vector|MakeVector 0.0 0.0 (* (Math|Trig|Sin(Radians) (Variables|Default|GetTime)) (Variables|Default|GetAmplitude)))) false false)
  (Transformation|AddRelativeRotation (Variables|Default|GetMagicCircle) (Math|Rotator|MakeRotator (* (Utilities|Time|GetWorldDeltaSeconds) -2.0) 0.0 0.0) false false))

(fn ConstructionScript)

(fn UpdateTime
  (params (A :type Float%20%28double-precision%29))
  (bind _output_get (Variables|Default|SetTime (+ A (Variables|Default|GetTime))))
  (if (>= _output_get (Variables|Default|Get2π))
    (Variables|Default|SetTime 0.0)))