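; BP_EffectActorBase is a base effect actor that animates its appearance and plays begin, impact and end sounds.
; On BeginPlay a timeline offsets height from InitializeLocation by Apex and scales the actor, playing ImpactSound on updates where the height curve dips below a threshold.
; When the timeline finishes, it starts sine and rotation movement.
; Tick applies CalculatedLocation and CalculatedRotation, which are computed outside these graphs.
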(event EventBeginPlay
  (Audio|PlaySoundatLocation (Variables|Default|GetBeginSound) (Transformation|GetActorLocation) "0, 0, 0" 1.0 1.0 0.0 0 0 0 0)
  (bind (_direction _newtrack_0 _scale) (Timeline|Timeline Play)
    (:Update
      (Transformation|SetActorLocation (+ (Variables|Default|GetInitializeLocation) (Math|Vector|MakeVector 0.0 0.0 (* _newtrack_0 (Variables|Default|GetApex)))) false false)
      (Transformation|SetActorScale3D (Math|Vector|MakeVector _scale _scale _scale))
      (if (< _newtrack_0 -0.1)
        (Audio|PlaySoundatLocation (Variables|Default|GetImpactSound) (Transformation|GetActorLocation) "0, 0, 0" 1.0 1.0 0.0 0 0 0 0)))
    (:Finished
      (Class|GASTEffectActor|StartSinMovement)
      (Class|GASTEffectActor|StartRotateMovement))))

(event EventDestroyed
  (Audio|PlaySoundatLocation (Variables|Default|GetEndSound) (Transformation|GetActorLocation) "0, 0, 0" 1.0 1.0 0.0 0 0 0 0))

(event EventTick
  (params (DeltaSeconds :type Float%20%28single-precision%29))
  (Transformation|SetActorLocation (Variables|Default|GetCalculatedLocation) false false)
  (Transformation|SetActorRotation (Variables|Default|GetCalculatedRotation)))

(fn ConstructionScript)